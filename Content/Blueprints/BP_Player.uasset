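; BP_Player is the player Blueprint, handling thruster effects and a fuel gauge on screen.
; On BeginPlay it creates the UMG_Player widget and adds it to the viewport.
; ActivateThrust and DeactivateThrust toggle the bottom, left or right thruster particle effect by direction index, only when its active state needs changing.
; ChangeFuel adds a delta to Fuel, clamps it to a normalized range and updates the widget's fuel bar.
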(event `self.ReceiveBeginPlay`
  (bind _returnvalue (`|CreateWidget` "/Game/UI/UMG_Player.UMG_Player_C"))
  (bind _output_get (set `self.UI` _returnvalue))
  (`UserWidget.AddToViewport` _output_get 0))

(event `ActivateThrust`
  (params (Direction :type Integer))
  ;[1 1 1] Particle Effect Activation Logic
  (switch `int` Direction
    (:`0`
      (if (not (`ActorComponent.IsActive` (`self.BottomThruster`)))
        (`ActorComponent.Activate` (`self.BottomThruster`) false)))
    (:`1`
      (if (not (`ActorComponent.IsActive` (`self.LeftThruster`)))
        (`ActorComponent.Activate` (`self.LeftThruster`) false)))
    (:`2`
      (if (not (`ActorComponent.IsActive` (`self.RightThruster`)))
        (`ActorComponent.Activate` (`self.RightThruster`) false)))))

(event `DeactivateThrust`
  (params (Direction :type Integer))
  ;[1 1 1] Particle Effect Activation Logic
  (switch `int` Direction
    (:`0`
      (if (`ActorComponent.IsActive` (`self.BottomThruster`))
        (`ActorComponent.Deactivate` (`self.BottomThruster`))))
    (:`1`
      (if (`ActorComponent.IsActive` (`self.LeftThruster`))
        (`ActorComponent.Deactivate` (`self.LeftThruster`))))
    (:`2`
      (if (`ActorComponent.IsActive` (`self.RightThruster`))
        (`ActorComponent.Deactivate` (`self.RightThruster`))))))

(event `ChangeFuel`
  (params (ChangeValue :type "Float (double-precision)"))
  (bind _output_get (set `self.Fuel` (`KismetMathLibrary.FClamp` (+ ChangeValue (`self.Fuel`)))))
  (`ProgressBar.SetPercent` (`/Game/UI/UMG_Player.FuelBar` (`self.UI`)) _output_get))

(fn `UserConstructionScript`)