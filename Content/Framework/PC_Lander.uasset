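; Player controller for a lander game that translates input into thrust, rotation and thruster effects on the player ship.
; On BeginPlay it caches the first BP_Player actor and initializes its fuel through ChangeFuel.
; While fuel remains, the Up axis applies force along the ship's up vector and the Right axis rotates it, both draining fuel over time.
; Separate action inputs toggle bottom, left and right thruster effects, independent of the fuel check.
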(event `self.ReceiveBeginPlay`
  ;[1 1 1] Store Player Ship Actor to Variable
  (bind _outactors (`GameplayStatics.GetAllActorsOfClass` "/Game/Blueprints/BP_Player.BP_Player_C"))
  (bind _output_get (set `self.PlayerShip` (`|GetArrayItem` _outactors)))
  (`/Game/Blueprints/BP_Player.ChangeFuel` _output_get 1.0))

(event `InputAxis|Up`
  (params (AxisValue :type "Float (single-precision)"))
  (bind _playership (`self.PlayerShip`))
  (bind _player (`/Game/Blueprints/BP_Player.Player` _playership))
  ;[1 1 1] Player Controls
  (if (> AxisValue 0.01)
    (if (> (`/Game/Blueprints/BP_Player.Fuel` _playership) 0.0)
      (`PrimitiveComponent.AddForce` _player (* (`SceneComponent.GetUpVector` _player) 10.0) "None" false)
      ;[1 1 1] Consume Fuel
      (`/Game/Blueprints/BP_Player.ChangeFuel` (`self.PlayerShip`) (* (`GameplayStatics.GetWorldDeltaSeconds`) -0.1) :!label _label))))

(event `InputAxis|Right`
  (params (AxisValue :type "Float (single-precision)"))
  (bind _playership (`self.PlayerShip`))
  (bind _player (`/Game/Blueprints/BP_Player.Player` _playership))
  (bind _returnvalue (> (`/Game/Blueprints/BP_Player.Fuel` _playership) 0.0))
  ;[1 1 1] Player Controls
  (if (> AxisValue 0.1)
    (if _returnvalue
      (`SceneComponent.K2_AddLocalRotation` _player (struct :`Pitch` -4.0) false false)
      (goto _label))
    (elif (< AxisValue -0.1)
      (if _returnvalue
        (`SceneComponent.K2_AddLocalRotation` _player (struct :`Pitch` 4.0) false false)
        (goto _label)))))

(event `InputAction|BottomThrust`
  (params (Key :type "Key Structure"))
  ;[1 1 1] Control Thruster Particle Effect
  (:`Pressed`
    (`/Game/Blueprints/BP_Player.ActivateThrust` (`self.PlayerShip`) 0))
  (:`Released`
    (`/Game/Blueprints/BP_Player.DeactivateThrust` (`self.PlayerShip`) 0)))

(event `InputAction|LeftThrust`
  (params (Key :type "Key Structure"))
  ;[1 1 1] Control Thruster Particle Effect
  (:`Pressed`
    (`/Game/Blueprints/BP_Player.ActivateThrust` (`self.PlayerShip`) 1))
  (:`Released`
    (`/Game/Blueprints/BP_Player.DeactivateThrust` (`self.PlayerShip`) 1)))

(event `InputAction|RightThrust`
  (params (Key :type "Key Structure"))
  ;[1 1 1] Control Thruster Particle Effect
  (:`Pressed`
    (`/Game/Blueprints/BP_Player.ActivateThrust` (`self.PlayerShip`) 2))
  (:`Released`
    (`/Game/Blueprints/BP_Player.DeactivateThrust` (`self.PlayerShip`) 2)))

(fn `UserConstructionScript`)