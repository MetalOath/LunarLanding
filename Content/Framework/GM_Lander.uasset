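; Game mode for a lander game that sets up play input and handles the win and lose outcomes of a landing attempt.
; BeginPlay hides the mouse cursor and switches to game-only input.
; GameOverWin and GameOverLose write a landed or crashed message to the bottom text of the HUD_Lander UI, then reload TheMoon level after a short delay.
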(event `self.ReceiveBeginPlay`
  (bind _returnvalue (`GameplayStatics.GetPlayerController` 0))
  (set `PlayerController.bShowMouseCursor` false _returnvalue)
  (`WidgetBlueprintLibrary.SetInputMode_GameOnly` _returnvalue))

(event `GameOverWin`
  (bind _ashud_lander (cast `/Game/Framework/HUD_Lander` (`PlayerController.GetHUD` (`GameplayStatics.GetPlayerController` 0))))
  (set `TextBlock.Text` "You Landed Safely!" (`/Game/UI/UMG_TheMoon.TextBottomScreen` (`/Game/Framework/HUD_Lander.UI` _ashud_lander)))
  (`KismetSystemLibrary.Delay` 2.0)
  (`GameplayStatics.OpenLevel` "TheMoon"))

(event `GameOverLose`
  (bind _ashud_lander (cast `/Game/Framework/HUD_Lander` (`PlayerController.GetHUD` (`GameplayStatics.GetPlayerController` 0))))
  (set `TextBlock.Text` "You Crashed!" (`/Game/UI/UMG_TheMoon.TextBottomScreen` (`/Game/Framework/HUD_Lander.UI` _ashud_lander)))
  (`KismetSystemLibrary.Delay` 2.0)
  (`GameplayStatics.OpenLevel` "TheMoon"))

(fn `UserConstructionScript`)